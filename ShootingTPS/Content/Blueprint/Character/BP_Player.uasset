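; BP_Player is the playable character, handling Enhanced Input movement, look and jump, weapon firing, damage and death.
; Attack plays a montage, then fires the child-actor BP_Weapon after a short delay, with a flag gating the cooldown.
; Damage lowers HP and broadcasts the change; death unpossesses, ragdolls the mesh, notifies the GameMode for respawn and destroys the actor after a delay.
; Health getters expose HP values, while IsAlive always returns false.
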(event `self.ReceiveBeginPlay`
  (`EnhancedInputSubsystemInterface.AddMappingContext` (pcsubsystem `EnhancedInputLocalPlayerSubsystem` (`GameplayStatics.GetPlayerController` 0)) "/Game/Input/IMC_Player.IMC_Player" 0 (struct))
  (bind _asbp_weapon (cast `/Game/Blueprint/Character/BP_Weapon` (`ChildActorComponent.ChildActor` (`self.Weapon`))))
  (set `self.EquippedWeapon` _asbp_weapon))

(event `EnhancedInput|/Game/Input/IA_PlayerMove`
  (params (ActionValue :type "Vector2D Structure") (ElapsedSeconds :type "Float (double-precision)") (TriggeredSeconds :type "Float (double-precision)") (InputAction :type "InputAction Object Reference" :default "/Game/Input/IA_PlayerMove.IA_PlayerMove"))
  (bind (_returnvalue_x _returnvalue_y) (`KismetMathLibrary.BreakVector2D` (`KismetMathLibrary.Normal2D` ActionValue)))
  (bind (_returnvalue_roll _returnvalue_pitch _returnvalue_yaw) (`KismetMathLibrary.BreakRotator` (`self.GetControlRotation`)))
  (bind _returnvalue (`KismetMathLibrary.MakeRotator` 0.0 0.0 _returnvalue_yaw))
  (:`Triggered`
    (if (not (`self.IsInteracting`))
      (`self.AddMovementInput` (`KismetMathLibrary.GetRightVector` _returnvalue) _returnvalue_x)
      (`self.AddMovementInput` (`KismetMathLibrary.GetForwardVector` _returnvalue) _returnvalue_y))))

(event `EnhancedInput|/Game/Input/IA_PlayerLook`
  (params (ActionValue :type "Vector2D Structure") (ElapsedSeconds :type "Float (double-precision)") (TriggeredSeconds :type "Float (double-precision)") (InputAction :type "InputAction Object Reference" :default "/Game/Input/IA_PlayerLook.IA_PlayerLook"))
  (bind (_returnvalue_x _returnvalue_y) (`KismetMathLibrary.BreakVector2D` (* ActionValue (`self.MouseSensitivity`))))
  (:`Triggered`
    (`self.AddControllerYawInput` _returnvalue_x)
    (`self.AddControllerPitchInput` _returnvalue_y)))

(event `EnhancedInput|/Game/Input/IA_PlayerJump`
  (params (ActionValue :type Boolean) (ElapsedSeconds :type "Float (double-precision)") (TriggeredSeconds :type "Float (double-precision)") (InputAction :type "InputAction Object Reference" :default "/Game/Input/IA_PlayerJump.IA_PlayerJump"))
  (:`Started`
    (switch `EMovementMode` (`CharacterMovementComponent.MovementMode` (`self.CharacterMovement`))
      (:`MOVE_Walking`
        (`self.Jump`))))
  (:`Completed`
    (`self.StopJumping`)))

(event `EnhancedInput|/Game/Input/IA_PlayerAttack`
  (params (ActionValue :type Boolean) (ElapsedSeconds :type "Float (double-precision)") (TriggeredSeconds :type "Float (double-precision)") (InputAction :type "InputAction Object Reference" :default "/Game/Input/IA_PlayerAttack.IA_PlayerAttack"))
  (:`Triggered`
    (`self.GunFire`)))

(event `GunFire`
  (if (`self.IsWeaponActivate`)
    (set `self.IsWeaponActivate` false)
    (`self.PlayAnimMontage` (`self.Attack Montage`))
    (`KismetSystemLibrary.Delay` 0.3)
    (`/Game/Blueprint/Character/BP_Weapon.FireWeapon` (`self.EquippedWeapon`))
    (`KismetSystemLibrary.Delay` 3.0)
    (set `self.IsWeaponActivate` true)))

(event `self.ReceiveAnyDamage`
  (params (Damage :type "Float (single-precision)") (DamageType :type "DamageType Object Reference") (InstigatedBy :type "Controller Object Reference") (DamageCauser :type "Actor Object Reference"))
  (bind _output_get (set `self.HP` (- (`self.HP`) Damage)))
  (`self.OnHPChange` _output_get)
  (if (<= _output_get 0.0)
    (`/Game/Blueprint/Interface/BPI_Die.OnDie`)))

(event `/Game/Blueprint/Interface/BPI_Die.OnDie`
  (bind _returnvalue (`GameplayStatics.GetGameMode`))
  (bind _mesh (`self.Mesh`))
  (`self.CharacterDie`)
  (`Controller.UnPossess` (`GameplayStatics.GetPlayerController` 0))
  (`PrimitiveComponent.SetCollisionProfileName` _mesh "Ragdoll" false)
  (`PrimitiveComponent.SetSimulatePhysics` _mesh true)
  (message `/Game/Blueprint/Interface/BPI_Respawner.RespawnPlayer` _returnvalue)
  (bind _respawntime (message `/Game/Blueprint/Interface/BPI_Respawner.GetRespawnTime` _returnvalue))
  (`KismetSystemLibrary.Delay` _respawntime)
  (`self.K2_DestroyActor`))

(fn `GetHealth`
  (returns (CurrentHealth :type "Float (double-precision)"))
  (return (`self.HP`)))

(fn `GetMaxHealth`
  (returns (MaxHealth :type "Float (double-precision)"))
  (return (`self.MaxHP`)))

(fn `IsAlive`
  (returns (IsAlive :type Boolean))
  (return false))

(fn `UserConstructionScript`)
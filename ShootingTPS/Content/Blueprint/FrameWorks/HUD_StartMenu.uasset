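; HUD Blueprint for the start menu that sets up the menu screen when play begins.
; BeginPlay blends player 0's view to a camera over a short time, then creates the start menu widget and adds it to the viewport.
; It then switches input to UI only and shows the mouse cursor.
; A disconnected lookup of the first CineCameraActor in the level never runs.
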(event `self.ReceiveBeginPlay`
  (bind _returnvalue (`GameplayStatics.GetPlayerController` 0))
  (`PlayerController.SetViewTargetWithBlend` _returnvalue (`self.Camera`) 0.5 "VTBlend_Linear" 0.0 false)
  (bind _returnvalue_2 (`|CreateWidget` "/Game/UI/WBP_StartMenu.WBP_StartMenu_C" _returnvalue))
  (`UserWidget.AddToViewport` _returnvalue_2 0)
  (`WidgetBlueprintLibrary.SetInputMode_UIOnlyEx` _returnvalue (`self.In Widget to Focus`) "DoNotLock" true)
  (set `PlayerController.bShowMouseCursor` true _returnvalue))

(fn `UserConstructionScript`)
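; Game state Blueprint that tracks the player's score and whether the game is over.
; On BeginPlay it casts the first player pawn to BP_Player and binds GameOver to its character death event, which sets the IsGameOver flag.
; AddScore accumulates points and broadcasts ScoreUpdated with the new total, while GetGameOverState exposes the flag to other objects.
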(event `self.ReceiveBeginPlay`
  (bind _asbp_player (cast `/Game/Blueprint/Character/BP_Player` (`GameplayStatics.GetPlayerPawn` 0)))
  (add `/Game/Blueprint/Character/BP_Player.CharacterDie` _asbp_player (delegate `GameOver`)))

(event `GameOver`
  (set `self.IsGameOver` true))

(event `/Game/Blueprint/Interface/BPI_Score.AddScore`
  (params (Point :type Integer))
  (bind _output_get (set `self.Score` (+ Point (`self.Score`))))
  (`self.ScoreUpdated` _output_get))

(fn `GetGameOverState`
  (returns (GameOver :type Boolean))
  (return (`self.IsGameOver`)))

(fn `UserConstructionScript`)
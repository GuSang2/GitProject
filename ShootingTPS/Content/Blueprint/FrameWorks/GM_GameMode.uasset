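; Game mode that serves as the access point for getting pooled enemies by type.
; On BeginPlay it caches the first BP_EnemyPool actor found in the level.
; GetEnemy switches on the enemy type to Chest or Slime helpers, which request an enemy at the given spawn transform from the matching sub-pool.
; Each helper checks validity first and returns the result cast to BP_PoolingEnemy_Base.
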(event `self.ReceiveBeginPlay`
  (bind _outactors (`GameplayStatics.GetAllActorsOfClass` "/Game/Blueprint/EnemySpawner/BP_EnemyPool.BP_EnemyPool_C"))
  (set `self.EnemyPool` (`|GetArrayItem` _outactors)))

(fn `GetEnemy`
  (params (Type :type "/Game/Blueprint/EnemySpawner/E_EnemyType Enum" :default "NewEnumerator0") (SpawnTransform :type "Transform Structure"))
  (returns (NewEnemy :type "/Game/Blueprint/Monster/BP_PoolingEnemy_Base Object Reference"))
  (switch `/Game/Blueprint/EnemySpawner/E_EnemyType` Type
    (:`NewEnumerator0`
      (bind _newenemy (`self.GetEnemy_Chest` SpawnTransform))
      (return _newenemy))
    (:`NewEnumerator1`
      (bind _newenemy_2 (`self.GetEnemy_Slime` SpawnTransform))
      (return _newenemy_2))))

(fn `GetEnemy_Chest`
  (params (SpawnTransform :type "Transform Structure"))
  (returns (NewEnemy :type "/Game/Blueprint/Monster/BP_PoolingEnemy_Base Object Reference"))
  (bind _enemypool (`self.EnemyPool`))
  (`/Engine/EditorBlueprintResources/StandardMacros.IsValid` _enemypool
    (:`Is Valid`
      (bind _newenemy (`/Game/Blueprint/EnemySpawner/AC_EnemyPool.GetEnemy` (`/Game/Blueprint/EnemySpawner/BP_EnemyPool.Pool_Chest` _enemypool) SpawnTransform))
      (bind _asbp_pooling_enemy_base (cast `/Game/Blueprint/Monster/BP_PoolingEnemy_Base` _newenemy))
      (return _asbp_pooling_enemy_base))))

(fn `GetEnemy_Slime`
  (params (SpawnTransform :type "Transform Structure"))
  (returns (NewEnemy :type "/Game/Blueprint/Monster/BP_PoolingEnemy_Base Object Reference"))
  (bind _pool_slime (`/Game/Blueprint/EnemySpawner/BP_EnemyPool.Pool_Slime` (`self.EnemyPool`)))
  (`/Engine/EditorBlueprintResources/StandardMacros.IsValid` _pool_slime
    (:`Is Valid`
      (bind _newenemy (`/Game/Blueprint/EnemySpawner/AC_EnemyPool.GetEnemy` _pool_slime SpawnTransform))
      (bind _asbp_pooling_enemy_base (cast `/Game/Blueprint/Monster/BP_PoolingEnemy_Base` _newenemy))
      (return _asbp_pooling_enemy_base))))

(fn `UserConstructionScript`)
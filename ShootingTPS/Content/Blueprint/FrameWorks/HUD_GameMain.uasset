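; HUD_GameMain is the main game HUD, which puts the in-game UI on screen when play begins.
; It creates a WBP_GameUI widget for the first player controller, stores it and adds it to the viewport.
; It then binds delegates to score updates on GS_GameBaseState and to character death on BP_Player, each reached through a cast that halts setup on failure.
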(event `self.ReceiveBeginPlay`
  (bind _returnvalue (`|CreateWidget` "/Game/UI/WBP_GameUI.WBP_GameUI_C" (`GameplayStatics.GetPlayerController` 0)))
  (bind _output_get (set `self.UI_Widget` _returnvalue))
  (`UserWidget.AddToViewport` _output_get 0)
  (bind _asgs_game_base_state (cast `/Game/Blueprint/FrameWorks/GS_GameBaseState` (`GameplayStatics.GetGameState`)))
  (add `/Game/Blueprint/FrameWorks/GS_GameBaseState.ScoreUpdated` _asgs_game_base_state (`|CreateDelegate` _output_get :!event `ScoreUpdate`))
  (bind _asbp_player (cast `/Game/Blueprint/Character/BP_Player` (`GameplayStatics.GetPlayerPawn` 0)))
  (add `/Game/Blueprint/Character/BP_Player.CharacterDie` _asbp_player (`|CreateDelegate` _output_get :!event `ShowGameOverPanel`)))

(fn `UserConstructionScript`)
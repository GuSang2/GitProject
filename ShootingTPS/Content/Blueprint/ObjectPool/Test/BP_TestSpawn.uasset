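; BP_TestSpawn is a test actor for the object pooling system that requests pooled objects on key presses.
; Pressing the 1 or 2 key calls GetObject on its ACPoolingObject component, and both keys behave identically.
; GetSpawnTransform supplies the world transform of the Area component as the spawn location.
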(event `Key|One`
  (params (Key :type "Key Structure"))
  (:`Pressed`
    (`/Game/Blueprint/ObjectPool/AC_PoolingObject.GetObject` (`self.AC_PoolingObject`) (`self.GetSpawnTransform`))))

(event `Key|Two`
  (params (Key :type "Key Structure"))
  (:`Pressed`
    (`/Game/Blueprint/ObjectPool/AC_PoolingObject.GetObject` (`self.AC_PoolingObject`) (`self.GetSpawnTransform`))))

(fn `GetSpawnTransform`
  (returns (SpawnTransform :type "Transform Structure"))
  (return (`SceneComponent.K2_GetComponentToWorld` (`self.Area`))))

(fn `UserConstructionScript`)